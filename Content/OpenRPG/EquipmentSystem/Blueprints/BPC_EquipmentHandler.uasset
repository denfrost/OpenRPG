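; Player controller component that equips and unequips items across eight RPG gear slots, linking slot widgets, inventory and stat handlers.
; EquipItem sets the slot's skeletal mesh on the pawn via master pose or socket, swapping occupied slots by unequipping and recursing.
; UnequipItem returns items to inventory, clears meshes and removes stat bonuses.
; A SaveGame restores gear on Initialize through EquipItem with index -1, which skips stat bonuses and inventory removal.
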(fn Initialize
  (params (EquipmentWidget :type WB%20Equipment%20Object%20Reference))
  (Variables|DoNotTouch!|SetEquipmentWidget EquipmentWidget)
  (bind _asbp_custom_player_controller (Utilities|Casting|CastToBP_CustomPlayerController (Components|GetOwner)))
  (bind _output_get (Variables|DoNotTouch!|SetPlayerControllerOwner _asbp_custom_player_controller))
  (bind _asbp_master_character (Utilities|Casting|CastToBP_MasterCharacter (Pawn|GetControlledPawn _output_get)))
  (Variables|DoNotTouch!|SetControlledPawn _asbp_master_character)
  (bind _output_get_2 (Variables|DoNotTouch!|SetEquipmentSlots (Utilities|Array|MakeArray (Variables|/Game/OpenRPG/EquipmentSystem/Widgets/WB_Equipment.WB_Equipment_C|GetHelmetSlot (Variables|DoNotTouch!|GetEquipmentWidget)) (Variables|/Game/OpenRPG/EquipmentSystem/Widgets/WB_Equipment.WB_Equipment_C|GetWeaponSlot (Variables|DoNotTouch!|GetEquipmentWidget)) (Variables|/Game/OpenRPG/EquipmentSystem/Widgets/WB_Equipment.WB_Equipment_C|GetArmorSlot (Variables|DoNotTouch!|GetEquipmentWidget)) (Variables|/Game/OpenRPG/EquipmentSystem/Widgets/WB_Equipment.WB_Equipment_C|GetShieldSlot (Variables|DoNotTouch!|GetEquipmentWidget)) (Variables|/Game/OpenRPG/EquipmentSystem/Widgets/WB_Equipment.WB_Equipment_C|GetRingSlot (Variables|DoNotTouch!|GetEquipmentWidget)) (Variables|/Game/OpenRPG/EquipmentSystem/Widgets/WB_Equipment.WB_Equipment_C|GetBeltSlot (Variables|DoNotTouch!|GetEquipmentWidget)) (Variables|/Game/OpenRPG/EquipmentSystem/Widgets/WB_Equipment.WB_Equipment_C|GetEarringsSlot (Variables|DoNotTouch!|GetEquipmentWidget)) (Variables|/Game/OpenRPG/EquipmentSystem/Widgets/WB_Equipment.WB_Equipment_C|GetBootsSlot (Variables|DoNotTouch!|GetEquipmentWidget))))) ; We have an array with all the slot widgets
  (for _array_element _output_get_2
    (Variables|/Game/OpenRPG/EquipmentSystem/Widgets/WB_EquipmentSlot.WB_EquipmentSlot_C|SetBPC_EquipmentHandler _array_element self) ; Set the red to this component
    (Default|Update _array_element) ; Updates the slot with an empty state
  )
  (Save/Load|LoadEquipment) ; If there is saved info it this will load it
  (return))

(fn EquipItem
  (params (NewItemInfo :type S%20Item%20Info%20Structure) (FromInventorySlot :type Integer))
  (bind _controlledpawn (Variables|DoNotTouch!|GetControlledPawn))
  (LocalVariables|SetLocalItemInfo NewItemInfo)
  (LocalVariables|SetLocalClickedSlot FromInventorySlot)
  (bind _output_get (LocalVariables|SetLocalWidgetSlot (Helpers|GetWidgetfromSlotType (.SlotType (Utilities|Struct|Breaks_EquipmentInfo (.EquipmentInfo (Utilities|Struct|Breaks_ItemInfo (LocalVariables|GetLocalItemInfo))))))))
  (if (Utilities|IsValidClass (.Class (Utilities|Struct|Breaks_ItemInfo (Variables|/Game/OpenRPG/EquipmentSystem/Widgets/WB_EquipmentSlot.WB_EquipmentSlot_C|GetItem _output_get)))) ; Is there already an item in the slot widget that we want to equip?
    (Default|RemoveAmountatIndex (Variables|/Game/OpenRPG/Shared/Blueprints/BP_CustomPlayerController.BP_CustomPlayerController_C|GetBPC_InventoryHandler (Variables|DoNotTouch!|GetPlayerControllerOwner)) (LocalVariables|GetLocalClickedSlot) 1) ; Removes for the swap
    (bind _success_ (Managment|UnequipItem (LocalVariables|GetLocalWidgetSlot) (LocalVariables|GetLocalClickedSlot))) ; There is already an item, so we have to unequip it
    (if _success_
      (Managment|EquipItem (LocalVariables|GetLocalItemInfo) -1) ; Now that the slot widget is clean, we call this function recursively
      (return)
      (else
        (Development|PrintString "Item cant be equipped" true true "(R=0.000000,G=0.660000,B=1.000000,A=1.000000)" 5.0)
        (return)))
    (else
      ;[0.08274 0.7685 1] Visual Equip
      (Utilities|IsValid (.SkeletalMesh (Utilities|Struct|Breaks_EquipmentInfo (.EquipmentInfo (Utilities|Struct|Breaks_ItemInfo (LocalVariables|GetLocalItemInfo))))) ; If it doesnt have visual equip mesh we just skip this
        (:Is%20Valid
          (bind _output_get_2 (LocalVariables|SetLocalMeshComponent (Utilities|Select :Index (.SlotType (Utilities|Struct|Breaks_EquipmentInfo (.EquipmentInfo (Utilities|Struct|Breaks_ItemInfo (LocalVariables|GetLocalItemInfo))))) :NewEnumerator3 (Variables|/Game/OpenRPG/Shared/Blueprints/BP_MasterCharacter.BP_MasterCharacter_C|GetWeapon _controlledpawn) :NewEnumerator1 (Variables|/Game/OpenRPG/Shared/Blueprints/BP_MasterCharacter.BP_MasterCharacter_C|GetArmor _controlledpawn) :NewEnumerator8 (Variables|/Game/OpenRPG/Shared/Blueprints/BP_MasterCharacter.BP_MasterCharacter_C|GetShield _controlledpawn) :NewEnumerator0 (Variables|/Game/OpenRPG/Shared/Blueprints/BP_MasterCharacter.BP_MasterCharacter_C|GetHelmet _controlledpawn) :NewEnumerator5 (Variables|/Game/OpenRPG/Shared/Blueprints/BP_MasterCharacter.BP_MasterCharacter_C|GetEarrings _controlledpawn) :NewEnumerator2 (Variables|/Game/OpenRPG/Shared/Blueprints/BP_MasterCharacter.BP_MasterCharacter_C|GetRing _controlledpawn) :NewEnumerator6 (Variables|/Game/OpenRPG/Shared/Blueprints/BP_MasterCharacter.BP_MasterCharacter_C|GetBelt _controlledpawn) :NewEnumerator4 (Variables|/Game/OpenRPG/Shared/Blueprints/BP_MasterCharacter.BP_MasterCharacter_C|GetBoots _controlledpawn))))
          (Class|SkinnedMeshComponent|SetSkeletalMesh _output_get_2 (.SkeletalMesh (Utilities|Struct|Breaks_EquipmentInfo (.EquipmentInfo (Utilities|Struct|Breaks_ItemInfo (LocalVariables|GetLocalItemInfo))))) true) ; Sets the skeletal mesh (the magic)
          (Transformation|SetRelativeTransform (LocalVariables|GetLocalMeshComponent) (.RelativeTransform (Utilities|Struct|Breaks_EquipmentInfo (.EquipmentInfo (Utilities|Struct|Breaks_ItemInfo (LocalVariables|GetLocalItemInfo))))) false false) ; This is only needed when we have to adjust manually the mesh in the skeleton socket
          (if (.UseCharacterSkeleton (Utilities|Struct|Breaks_EquipmentInfo (.EquipmentInfo (Utilities|Struct|Breaks_ItemInfo (LocalVariables|GetLocalItemInfo)))))
            (Class|SkinnedMeshComponent|SetMasterPoseComponent (LocalVariables|GetLocalMeshComponent) (Variables|/Script/Engine.Character|GetMesh (Variables|DoNotTouch!|GetControlledPawn))) ; If the equipment mesh uses the same skeleton as the character, this function will adjust it, so it will follow the animations and so on, its like AttachToComponent but automatically
            (else
              (Transformation|AttachComponentToComponent (LocalVariables|GetLocalMeshComponent) (Variables|/Script/Engine.Character|GetMesh (Variables|DoNotTouch!|GetControlledPawn)) (.SocketName (Utilities|Struct|Breaks_EquipmentInfo (.EquipmentInfo (Utilities|Struct|Breaks_ItemInfo (LocalVariables|GetLocalItemInfo))))) "KeepRelative" "KeepRelative" "KeepRelative" true) ; Attach the socket to the one that we have created in the skeleton (you can use a bone too if you want), so it will follow the animations
            )))
        (:Is%20Not%20Valid
          _))
      (Default|Update (LocalVariables|GetLocalWidgetSlot) (LocalVariables|GetLocalItemInfo)) ; Updates the slot widget
      (if (!= (LocalVariables|GetLocalClickedSlot) -1)
        (Default|AddStatBonus (Variables|/Game/OpenRPG/Shared/Blueprints/BP_CustomPlayerController.BP_CustomPlayerController_C|GetBPC_StatsHandler (Variables|DoNotTouch!|GetPlayerControllerOwner)) (Utilities|Struct|Breaks_EquipmentInfo (.EquipmentInfo (Utilities|Struct|Breaks_ItemInfo (LocalVariables|GetLocalItemInfo)))))
        (Default|RemoveAmountatIndex (Variables|/Game/OpenRPG/Shared/Blueprints/BP_CustomPlayerController.BP_CustomPlayerController_C|GetBPC_InventoryHandler (Variables|DoNotTouch!|GetPlayerControllerOwner)) (LocalVariables|GetLocalClickedSlot) 1)
        (return)
        (else
          (return))))))

(fn UnequipItem
  (params (SlotWidget :type WB%20Equipment%20Slot%20Object%20Reference) (ToSpecificInventoryIndex :type Integer))
  (bind _controlledpawn (Variables|DoNotTouch!|GetControlledPawn))
  (bind _output_get (LocalVariables|SetLocalSlotWidget SlotWidget))
  (LocalVariables|SetLocalSpecificIndex ToSpecificInventoryIndex)
  (LocalVariables|SetLocalItemInfo (Variables|/Game/OpenRPG/EquipmentSystem/Widgets/WB_EquipmentSlot.WB_EquipmentSlot_C|GetItem _output_get))
  (if (!= (LocalVariables|GetLocalSpecificIndex) -1) ; If the index is != -1 it means we are dragging a slot from the equipment window
    (if (Default|IsSlotEmpty? (Variables|/Game/OpenRPG/Shared/Blueprints/BP_CustomPlayerController.BP_CustomPlayerController_C|GetBPC_InventoryHandler (Variables|DoNotTouch!|GetPlayerControllerOwner)) (LocalVariables|GetLocalSpecificIndex))
      (bind _success_ (Default|AddItematIndex (Variables|/Game/OpenRPG/Shared/Blueprints/BP_CustomPlayerController.BP_CustomPlayerController_C|GetBPC_InventoryHandler (Variables|DoNotTouch!|GetPlayerControllerOwner)) (LocalVariables|GetLocalItemInfo) (LocalVariables|GetLocalSpecificIndex) 1)) ; We can add to the slot because its empty
      (if _success_
        (Utilities|IsValid (.SkeletalMesh (Utilities|Struct|Breaks_EquipmentInfo (.EquipmentInfo (Utilities|Struct|Breaks_ItemInfo (LocalVariables|GetLocalItemInfo))))) :!label _label ; If it doesnt have visual equip mesh we just skip this
          (:Is%20Valid
            (bind _output_get_2 (LocalVariables|SetLocalMeshComponent (Utilities|Select :Index (.SlotType (Utilities|Struct|Breaks_EquipmentInfo (.EquipmentInfo (Utilities|Struct|Breaks_ItemInfo (LocalVariables|GetLocalItemInfo))))) :NewEnumerator3 (Variables|/Game/OpenRPG/Shared/Blueprints/BP_MasterCharacter.BP_MasterCharacter_C|GetWeapon _controlledpawn) :NewEnumerator1 (Variables|/Game/OpenRPG/Shared/Blueprints/BP_MasterCharacter.BP_MasterCharacter_C|GetArmor _controlledpawn) :NewEnumerator8 (Variables|/Game/OpenRPG/Shared/Blueprints/BP_MasterCharacter.BP_MasterCharacter_C|GetShield _controlledpawn) :NewEnumerator0 (Variables|/Game/OpenRPG/Shared/Blueprints/BP_MasterCharacter.BP_MasterCharacter_C|GetHelmet _controlledpawn) :NewEnumerator5 (Variables|/Game/OpenRPG/Shared/Blueprints/BP_MasterCharacter.BP_MasterCharacter_C|GetEarrings _controlledpawn) :NewEnumerator2 (Variables|/Game/OpenRPG/Shared/Blueprints/BP_MasterCharacter.BP_MasterCharacter_C|GetRing _controlledpawn) :NewEnumerator6 (Variables|/Game/OpenRPG/Shared/Blueprints/BP_MasterCharacter.BP_MasterCharacter_C|GetBelt _controlledpawn) :NewEnumerator4 (Variables|/Game/OpenRPG/Shared/Blueprints/BP_MasterCharacter.BP_MasterCharacter_C|GetBoots _controlledpawn))))
            (Class|SkinnedMeshComponent|SetSkeletalMesh _output_get_2 0 true))
          (:Is%20Not%20Valid
            _))
        (Default|Update (LocalVariables|GetLocalSlotWidget)) ; Finally we clear the slot widget and return success
        (Default|RemoveStatBonuses (Variables|/Game/OpenRPG/Shared/Blueprints/BP_CustomPlayerController.BP_CustomPlayerController_C|GetBPC_StatsHandler (Variables|DoNotTouch!|GetPlayerControllerOwner)) (Utilities|Struct|Breaks_EquipmentInfo (.EquipmentInfo (Utilities|Struct|Breaks_ItemInfo (LocalVariables|GetLocalItemInfo)))))
        (return true)
        (else
          _)))
    (else
      (bind _success__2 (Default|AddIItem(Public) (Variables|/Game/OpenRPG/Shared/Blueprints/BP_CustomPlayerController.BP_CustomPlayerController_C|GetBPC_InventoryHandler (Variables|DoNotTouch!|GetPlayerControllerOwner)) (LocalVariables|GetLocalItemInfo) 1)) ; Unequip in the firts empty slot
      (if _success__2
        (goto _label)
        (else
          _))))
  (Development|PrintString "Item cant be unequipped" true true "(R=0.000000,G=0.660000,B=1.000000,A=1.000000)" 5.0) ; Inventory full or the inventory slot that we are dropping isnt empty
  (return false))

(fn LoadEquipment
  (bind _returnvalue (SaveGame|DoesSaveGameExist (Variables|Save/Load|GetEquipmentSlot)))
  (if _returnvalue
    (Utilities|IsValid (Variables|Save/Load|GetEquipmentSaveObject)
      (:Is%20Valid
        _)
      (:Is%20Not%20Valid
        (bind _returnvalue_2 (SaveGame|LoadGamefromSlot (Variables|Save/Load|GetEquipmentSlot)))
        (bind _asequipment_save (Utilities|Casting|CastToEquipmentSave _returnvalue_2))
        (Variables|Save/Load|SetEquipmentSaveObject _asequipment_save)))
    (for _array_element (Variables|/Game/OpenRPG/EquipmentSystem/Blueprints/EquipmentSave.EquipmentSave_C|GetSavedEquipmentItems (Variables|Save/Load|GetEquipmentSaveObject))
      (if (Utilities|IsValidClass (.Class (Utilities|Struct|Breaks_ItemInfo _array_element)))
        (Managment|EquipItem _array_element -1)))
    (return true)
    (else
      (return false))))

(fn SaveEquipment
  (Utilities|IsValid (Variables|Save/Load|GetEquipmentSaveObject)
    (:Is%20Valid
      _)
    (:Is%20Not%20Valid
      (bind _returnvalue (SaveGame|CreateSaveGameObject "/Game/OpenRPG/EquipmentSystem/Blueprints/EquipmentSave.EquipmentSave_C"))
      (Variables|Save/Load|SetEquipmentSaveObject _returnvalue)))
  (Utilities|Array|Clear (Variables|/Game/OpenRPG/EquipmentSystem/Blueprints/EquipmentSave.EquipmentSave_C|GetSavedEquipmentItems (Variables|Save/Load|GetEquipmentSaveObject)))
  (for _array_element (Variables|DoNotTouch!|GetEquipmentSlots)
    (Utilities|Array|Add (Variables|/Game/OpenRPG/EquipmentSystem/Blueprints/EquipmentSave.EquipmentSave_C|GetSavedEquipmentItems (Variables|Save/Load|GetEquipmentSaveObject)) (Variables|/Game/OpenRPG/EquipmentSystem/Widgets/WB_EquipmentSlot.WB_EquipmentSlot_C|GetItem _array_element)))
  (SaveGame|SaveGametoSlot (Variables|Save/Load|GetEquipmentSaveObject) (Variables|Save/Load|GetEquipmentSlot))
  (return))

(fn GetWidgetfromSlotType
  (params (SlotType :type e_EquipmentSlot%20Enum :default "NewEnumerator3"))
  (LocalVariables|SetLocalSlotType SlotType)
  (bind _array_element (Utilities|Array|ForEachLoopwithBreak (Variables|DoNotTouch!|GetEquipmentSlots) :!label _label)
    (:LoopBody
      (if (Utilities|Enum|Equal(Enum) (Variables|/Game/OpenRPG/EquipmentSystem/Widgets/WB_EquipmentSlot.WB_EquipmentSlot_C|GetSlotType _array_element) (LocalVariables|GetLocalSlotType))
        (LocalVariables|SetLocalWidget _array_element)
        (goto _label Break)))
    (:Completed
      (return (LocalVariables|GetLocalWidget)))))

(fn ToggleEquipmentVisibility
  (bind _equipmentwidget (Variables|DoNotTouch!|GetEquipmentWidget))
  (bind _returnvalue (Widget|IsVisible _equipmentwidget))
  (bind _returnvalue_2 (select _returnvalue "Hidden" "Visible"))
  (Widget|SetVisibility (Variables|DoNotTouch!|GetEquipmentWidget) _returnvalue_2)
  (Widget|SetIsEnabled (Variables|DoNotTouch!|GetEquipmentWidget) (Utilities|Select :Index _returnvalue_2 :Visible false :Collapsed false :Hidden true :HitTestInvisible false :SelfHitTestInvisible false))
  (return))