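; Player controller component that manages the player's learned skills, skill points and spell casting in the RPG.
; Initialize loads saved skills or uses the default list, spawning each as a spell actor at its stage.
; UseSkill casts only when no spell is active, and casting disables other skill hotkeys until it ends.
; SaveSkills persists skills and points to a save slot; LearnSkill and IsSkillLearned are empty stubs.
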(event Custom|UseSkill
  (params (Skill :type BP%20Base%20Skill%20Object%20Reference) (HotKey :type WB%20Hot%20Key%20Object%20Reference))
  (Utilities|IsValid (Variables|Default|GetCurrentSpell)
    (:Is%20Not%20Valid
      (Variables|/Game/OpenRPG/SkillSystem/Blueprints/BP_BaseSkill.BP_BaseSkill_C|SetHotKey Skill HotKey)
      (Default|TrySpellCast Skill))))

(fn SpendSkillPoint
  (params (Index :type Integer))
  (LocalVariables|SetLocalIndex Index)
  (if (> (Variables|Default|GetSkillPoints) 0)
    (Variables|Default|SetSkillPoints (- (Variables|Default|GetSkillPoints) 1))
    (Variables|Default|SetSpentSkillPoints (+ (Variables|Default|GetSpentSkillPoints) 1))
    (LocalVariables|SetLocalSkill (Utilities|Array|Get(acopy) (Variables|Default|GetLearnedSkills) (LocalVariables|GetLocalIndex)))
    (return)))

(fn SaveSkills
  (Utilities|IsValid (Variables|Default|GetSkillsSaveObject)
    (:Is%20Valid
      _)
    (:Is%20Not%20Valid
      (bind _returnvalue (SaveGame|CreateSaveGameObject "/Game/OpenRPG/SkillSystem/Blueprints/SkillSave.SkillSave_C"))
      (Variables|Default|SetSkillsSaveObject _returnvalue)))
  (Variables|/Game/OpenRPG/SkillSystem/Blueprints/SkillSave.SkillSave_C|SetSavedSkills (Variables|Default|GetSkillsSaveObject) (Variables|Default|GetLearnedSkills))
  (Variables|/Game/OpenRPG/SkillSystem/Blueprints/SkillSave.SkillSave_C|SetSkillPoints (Variables|Default|GetSkillsSaveObject) (Variables|Default|GetSkillPoints))
  (Variables|/Game/OpenRPG/SkillSystem/Blueprints/SkillSave.SkillSave_C|SetSpentSkillPoints (Variables|Default|GetSkillsSaveObject) (Variables|Default|GetSpentSkillPoints))
  (SaveGame|SaveGametoSlot (Variables|Default|GetSkillsSaveObject) (Variables|Default|GetSkillsSave))
  (return))

(fn LoadSkills
  (bind _returnvalue (SaveGame|DoesSaveGameExist (Variables|Default|GetSkillsSave)))
  (if _returnvalue
    (Utilities|IsValid (Variables|Default|GetSkillsSaveObject)
      (:Is%20Valid
        _)
      (:Is%20Not%20Valid
        (bind _returnvalue_2 (SaveGame|LoadGamefromSlot (Variables|Default|GetSkillsSave)))
        (bind _asskill_save (Utilities|Casting|CastToSkillSave _returnvalue_2)
          (:then
            (Variables|Default|SetSkillsSaveObject _asskill_save))
          (:CastFailed
            (return false)))))
    (Variables|Default|SetLearnedSkills (Variables|/Game/OpenRPG/SkillSystem/Blueprints/SkillSave.SkillSave_C|GetSavedSkills (Variables|Default|GetSkillsSaveObject)))
    (Variables|Default|SetSkillPoints (Variables|/Game/OpenRPG/SkillSystem/Blueprints/SkillSave.SkillSave_C|GetSkillPoints (Variables|Default|GetSkillsSaveObject)))
    (Variables|Default|SetSpentSkillPoints (Variables|/Game/OpenRPG/SkillSystem/Blueprints/SkillSave.SkillSave_C|GetSpentSkillPoints (Variables|Default|GetSkillsSaveObject)))
    (for _array_element (Variables|Default|GetLearnedSkills)
      (bind _returnvalue_3 (Game|SpawnActorfromClass (.Skill (Utilities|Struct|Breaks_Skill _array_element)) (Math|Transform|MakeTransform "0, 0, 0" "0, 0, 0" "1,1,1") "AlwaysSpawn" 0 self (.CurrentStageIndex (Utilities|Struct|Breaks_Skill _array_element)) 0))
      (Utilities|Array|Add (Variables|Default|GetSpells) _returnvalue_3))
    (return true)
    (else
      (return false))))

(fn Initialize
  (bind _asbp_custom_player_controller (Utilities|Casting|CastToBP_CustomPlayerController (Components|GetOwner)))
  (bind _output_get (Variables|Default|SetPlayerControllerOwner _asbp_custom_player_controller))
  (Variables|Default|SetControlledPawn (Variables|/Game/OpenRPG/Shared/Blueprints/BP_CustomPlayerController.BP_CustomPlayerController_C|GetControlledPawn _output_get))
  (bind _success_ (CallFunction|LoadSkills))
  (if _success_
    (return)
    (else
      (for _array_element (Variables|Default|GetLearnedSkills)
        (bind _returnvalue (Game|SpawnActorfromClass (.Skill (Utilities|Struct|Breaks_Skill _array_element)) (Math|Transform|MakeTransform "0, 0, 0" "0, 0, 0" "1,1,1") "AlwaysSpawn" 0 self (.CurrentStageIndex (Utilities|Struct|Breaks_Skill _array_element)) 0))
        (Utilities|Array|Add (Variables|Default|GetSpells) _returnvalue))
      (return))))

(fn BeginSpellCast
  (params (Spell :type BP%20Base%20Skill%20Object%20Reference))
  (Variables|Default|SetCurrentSpell Spell)
  (for _array_element (Variables|/Game/OpenRPG/HotKeyBarSystem/Blueprints/BPC_HoyKeyBarHandler.BPC_HoyKeyBarHandler_C|GetHotKeys (Variables|/Game/OpenRPG/Shared/Blueprints/BP_CustomPlayerController.BP_CustomPlayerController_C|GetBPC_HoyKeyBarHandler (Variables|Default|GetPlayerControllerOwner)))
    (if (and (Default|HasSkill? _array_element) (!= (Variables|/Game/OpenRPG/HotKeyBarSystem/Widgets/WB_HotKey.WB_HotKey_C|GetSpell _array_element) (Variables|Default|GetCurrentSpell)))
      (Default|DisableHotKey _array_element)))
  (return))

(fn EndSpellCast
  (params (Spell :type BP%20Base%20Skill%20Object%20Reference))
  (LocalVariables|SetLocalSpell Spell)
  (Variables|Default|SetCurrentSpell 0)
  (for _array_element (Variables|/Game/OpenRPG/HotKeyBarSystem/Blueprints/BPC_HoyKeyBarHandler.BPC_HoyKeyBarHandler_C|GetHotKeys (Variables|/Game/OpenRPG/Shared/Blueprints/BP_CustomPlayerController.BP_CustomPlayerController_C|GetBPC_HoyKeyBarHandler (Variables|Default|GetPlayerControllerOwner)))
    (if (and (Default|HasSkill? _array_element) (!= (Variables|/Game/OpenRPG/HotKeyBarSystem/Widgets/WB_HotKey.WB_HotKey_C|GetSpell _array_element) (LocalVariables|GetLocalSpell)))
      (Default|EnableHotKey _array_element)))
  (return))

(fn LearnSkill)

(fn IsSkillLearned?)

(fn GetSkill
  (params (Class :type BP%20Base%20Skill%20Class%20Reference))
  (LocalVariables|SetLocalClass Class)
  (bind _array_element (Utilities|Array|ForEachLoopwithBreak (Variables|Default|GetSpells) :!label _label)
    (:LoopBody
      (if (== (Utilities|GetClass _array_element) (LocalVariables|GetLocalClass))
        (LocalVariables|SetLocalSpell _array_element)
        (goto _label Break)))
    (:Completed
      (return (LocalVariables|GetLocalSpell)))))