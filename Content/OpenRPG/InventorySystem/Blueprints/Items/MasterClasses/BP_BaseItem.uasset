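; Base item Blueprint for the OpenRPG inventory system, the parent class that defines what happens when an item is used.
; UseItem stores the clicked slot and PlayerController and plays the item's optional used sound; type-level children override it with shared logic and should finish by destroying the spawned item.
; OnItemUsed is the override point for per-item effects, and here only prints a debug message with the item name.
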(event Custom|UseItem
  (params (Clicked%20Slot%20Index :type Integer) (PlayerController :type BP%20Custom%20Player%20Controller%20Object%20Reference))
  (bind _iteminfo (Variables|Default|GetItemInfo))
  (bind _onusedsound (Utilities|Struct|Breaks_ItemInfo _iteminfo))
  ;[0.1043 1 0.1512] This event must be overriden in the child BaseClasses, it will define shared logic when an item from the same type is used. For example, consumable items decrease its amount by 1, while equipment items are handled with the EquipItem function. See the examples to get a better idea. It should always finish destroying the spawned item once it has executed the logic
  (Variables|Default|SetClickedSlotIndex Clicked%20Slot%20Index)
  (Variables|Default|SetPlayerController PlayerController)
  (Utilities|IsValid _onusedsound
    (:Is%20Valid
      (Audio|PlaySound2D _onusedsound))))

(event Custom|OnItemUsed
  ;[0.05805 0.4849 1] So here is the potential of this implementation, you can set what each item does when used, just overriding this event in the child classes, with access to the player controller :D
  (Development|PrintString (Utilities|String|Append "Item " (Utilities|String|ToString(Name) (.Name (Utilities|Struct|Breaks_ItemInfo (Variables|Default|GetItemInfo)))) " has been used!") true true "(R=0.000000,G=0.660000,B=1.000000,A=1.000000)" 5.0) ; Just debug
)

(fn ConstructionScript)