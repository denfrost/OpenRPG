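; BP_PickUp is a world item pickup actor holding an ItemInfo and Amount.
; The construction script loads ItemInfo from DT_Items unless ItemID is -1 for custom info, then applies mesh, scale and interaction radius.
; Sphere overlap registers it in the character's NearbyItems and toggles a name/amount prompt widget.
; OnPickUp, called by the PlayerController, adds it to the inventory and destroys the actor only on success.
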(event OnComponentBeginOverlap(Colision)
  (params (OverlappedComponent :type Primitive%20Component%20Object%20Reference) (OtherActor :type Actor%20Object%20Reference) (OtherComp :type Primitive%20Component%20Object%20Reference) (OtherBodyIndex :type Integer) (bFromSweep :type Boolean) (SweepResult :type Hit%20Result%20Structure%20%28by%20ref%29))
  ;[0.9062 0.3879 0.2239] This Actor is just a simple way to interact with items in the world. It accepts Amount and an ItemID, and if it is != -1 the Construction Script will take the proper info from the items DataTable (if it is -1 it means we want to plug a custom ItemInfo, see the Drop function in the InventoryComponent to get an idea).
  (bind _asbp_master_character (Utilities|Casting|CastToBP_MasterCharacter OtherActor))
  (Utilities|Array|Add (Variables|/Game/OpenRPG/Shared/Blueprints/BP_MasterCharacter.BP_MasterCharacter_C|GetNearbyItems _asbp_master_character) self)
  (Rendering|SetVisibility (Variables|Default|GetText) true false))

(event OnComponentEndOverlap(Colision)
  (params (OverlappedComponent :type Primitive%20Component%20Object%20Reference) (OtherActor :type Actor%20Object%20Reference) (OtherComp :type Primitive%20Component%20Object%20Reference) (OtherBodyIndex :type Integer))
  ;[0.9062 0.3879 0.2239] This Actor is just a simple way to interact with items in the world. It accepts Amount and an ItemID, and if it is != -1 the Construction Script will take the proper info from the items DataTable (if it is -1 it means we want to plug a custom ItemInfo, see the Drop function in the InventoryComponent to get an idea).
  (bind _asbp_master_character (Utilities|Casting|CastToBP_MasterCharacter OtherActor))
  (Utilities|Array|RemoveItem (Variables|/Game/OpenRPG/Shared/Blueprints/BP_MasterCharacter.BP_MasterCharacter_C|GetNearbyItems _asbp_master_character) self)
  (Rendering|SetVisibility (Variables|Default|GetText) false false))

(event Custom|OnPickUp
  (params (PlayerController :type BP%20Custom%20Player%20Controller%20Object%20Reference))
  ;[0.9062 0.3879 0.2239] This Actor is just a simple way to interact with items in the world. It accepts Amount and an ItemID, and if it is != -1 the Construction Script will take the proper info from the items DataTable (if it is -1 it means we want to plug a custom ItemInfo, see the Drop function in the InventoryComponent to get an idea).
  (bind _output_get (Variables|Default|SetPlayerController PlayerController))
  (bind _success_ (Default|AddIItem(Public) (Variables|/Game/OpenRPG/Shared/Blueprints/BP_CustomPlayerController.BP_CustomPlayerController_C|GetBPC_InventoryHandler _output_get) (Variables|Default|GetItemInfo) (Variables|Default|GetAmount))) ; We try to add the item
  (if _success_ ; Not enough space?
    (Utilities|Array|RemoveItem (Variables|/Game/OpenRPG/Shared/Blueprints/BP_MasterCharacter.BP_MasterCharacter_C|GetNearbyItems (Variables|/Game/OpenRPG/Shared/Blueprints/BP_CustomPlayerController.BP_CustomPlayerController_C|GetControlledPawn (Variables|Default|GetPlayerController))) self) ; Updates the nearby items in the player character
    (Actor|DestroyActor) ; Destroy self
  ))

(event EventBeginPlay
  ;[0.9062 0.3879 0.2239] This Actor is just a simple way to interact with items in the world. It accepts Amount and an ItemID, and if it is != -1 the Construction Script will take the proper info from the items DataTable (if it is -1 it means we want to plug a custom ItemInfo, see the Drop function in the InventoryComponent to get an idea).
  (bind _aswb_interact_text (Utilities|Casting|CastToWB_InteractText (UserInterface|GetUserWidgetObject (Variables|Default|GetText)))) ; Get the widget from the component
  (Default|Initialize _aswb_interact_text (Utilities|Text|FormatText "{Name} x{Amount}" (Utilities|Text|ToText(Name) (.Name (Utilities|Struct|Breaks_ItemInfo (Variables|Default|GetItemInfo)))) (Variables|Default|GetAmount)) "Press [E] to interact!") ; Initialize with custom data from this actor
  (CallFunction|SetVisualProperties))

(fn ConstructionScript
  (if (!= (Variables|Default|GetItemID) -1)
    (bind _returnvalue (Utilities|GetDataTableRow "/Game/OpenRPG/InventorySystem/Blueprints/Items/DT_Items.DT_Items" (Utilities|String|StringToName (Utilities|String|ToString(Integer) (Variables|Default|GetItemID)))) ; Get the info from the data table
      (:then
        (Variables|Default|SetItemInfo _returnvalue)
        (CallFunction|SetVisualProperties)))))

(fn SetVisualProperties
  (bind _iteminfo (Variables|Default|GetItemInfo))
  (bind _iteminfo_2 (Variables|Default|GetItemInfo))
  (bind (_onusedsound _worldmesh _meshscale _interactradius) (Utilities|Struct|Breaks_ItemInfo _iteminfo))
  (bind _worldmesh_2 (Utilities|Struct|Breaks_ItemInfo _iteminfo_2))
  ;[0.4047 0.1297 1] This takes the mesh, the scale and the interaction sphere radious and set it
  (Components|StaticMesh|SetStaticMesh (Variables|Default|GetDefaultMesh) _worldmesh_2)
  (Rendering|Material|SetMaterial (Variables|Default|GetDefaultMesh) 0 (Rendering|Material|GetMaterial _worldmesh_2 0))
  (Transformation|SetWorldScale3D (Variables|Default|GetDefaultMesh) _meshscale)
  (Components|Sphere|SetSphereRadius (Variables|Default|GetColision) _interactradius false)
  (return))